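; BP_Spaceship is the player's ship: it turns to face the mouse cursor and loses lives when hit by asteroids.
; Every tick it traces under the cursor and sets only its yaw toward the impact point, zeroing pitch and roll.
; Hitting an Asteroid destroys it, decrements CurrentLives, updates the hearts in WBP_Lives found by class lookup, and quits the game when none remain.
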(event EventBeginPlay)

(event EventTick
  (params (DeltaSeconds :type Float%20%28single-precision%29))
  (Transformation|SetActorRotation (Math|Rotator|MakeRotator 0.0 0.0 (.Yaw (Math|Rotator|BreakRotator (Math|Rotator|FindLookatRotation (Transformation|GetActorLocation) (.ImpactPoint (Collision|BreakHitResult (.HitResult (Game|Player|GetHitResultUnderCursorbyChannel (Game|GetPlayerController 0) "TraceTypeQuery1" true))))))))))

(event Collision|EventHit
  (params (MyComp :type Primitive%20Component%20Object%20Reference) (Other :type Actor%20Object%20Reference) (OtherComp :type Primitive%20Component%20Object%20Reference) (bSelfMoved :type Boolean) (HitLocation :type Vector :default "0, 0, 0") (HitNormal :type Vector :default "0, 0, 0") (NormalImpulse :type Vector :default "0, 0, 0") (Hit :type Hit%20Result%20Structure%20%28by%20ref%29))
  (bind _asasteroid (Utilities|Casting|CastToAsteroid Other))
  (Actor|DestroyActor _asasteroid)
  (bind _output_get (Variables|Default|SetCurrentLives (Variables|Default|GetCurrentLives)))
  (bind _result (Math|Integer|DecrementInt _output_get)
    (:%20%20
      (bind _foundwidgets (Widget|GetAllWidgetsOfClass "/Game/Core/WBP_Lives.WBP_Lives_C" true))
      (Default|UpdateHearts _foundwidgets _result)
      (if (<= _result 0)
        (Game|QuitGame 0 "Quit" false)))))

(fn ConstructionScript)